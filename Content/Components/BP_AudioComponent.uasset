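; Audio component for tanks that plays idle and movement loops for the player pawn or an enemy tank, plus a death sound.
; On BeginPlay it casts its owner to BP_PlayerPawn or BP_BaseTank and binds to that pawn's movement mode change event.
; Each change fades out the previous sound and fades in a newly spawned attached one, using attenuation for enemies only.
; The death sound plays in 2D for any owner.
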(event `Player Movement Sound Updated`
  (`self.Play Current Player  Movement State Sound`))

(event `self.ReceiveBeginPlay`
  (bind _asbp_player_pawn (cast `/Game/Player/Pawns/BP_PlayerPawn` (`self.GetOwner`))
    (:`then`
      (bind _output_get (set `self.As BP Player Pawn` _asbp_player_pawn))
      (add `/Game/Player/Pawns/BP_PlayerPawn.Player Movement Mode Changed` _output_get (delegate `Player Movement Sound Updated`)))
    (:`CastFailed`
      (bind _asbp_base_tank (cast `/Game/AI/Pawns/TankEnemies/BP_BaseTank` (`self.GetOwner`))
        (:`then`
          (bind _output_get_2 (set `self.As BP Base Tank` _asbp_base_tank))
          (add `/Game/AI/Pawns/TankEnemies/BP_BaseTank.Enemy Tank Movement Mode Changed` _output_get_2 (delegate `Enemy Movment Sound Updated`)))
        (:`CastFailed`
          (`KismetSystemLibrary.PrintString` "BP_AudioComponent -  Play Movement Sound: Cast to any pawn to atattempt to play movement sound has failed"))))))

(event `Enemy Movment Sound Updated`
  (`self.Play Current Enemy  Movement State Sound`))

(event `self.ReceiveTick`
  (params (DeltaSeconds :type "Float (single-precision)")))

(fn `Play Current Enemy  Movement State Sound`
  (switch `/Game/Player/FSM/EMovementMode` (`/Game/AI/Pawns/TankEnemies/BP_BaseTank.Current Movement Mode` (`self.As BP Base Tank`))
    (:`NewEnumerator0`
      (`AudioComponent.FadeOut` (`self.Moving Sound Component`) 0.5 0.0 "Linear")
      (bind _returnvalue (`GameplayStatics.SpawnSoundAttached` (`self.Idle Sound`) (`Actor.RootComponent` (`self.GetOwner`)) "None" (0.0 0.0 0.0) (struct) "KeepRelativeOffset" false 1.0 1.0 0.0 "/Game/Audio/SoundAttenuators/SA_EnemyTankMovement.SA_EnemyTankMovement" null))
      (bind _output_get (set `self.Idle Sound Component` _returnvalue))
      (`AudioComponent.FadeIn` _output_get 0.5 1.0 0.0 "Linear")
      (`KismetSystemLibrary.PrintString` "IDLE SOUND STATE"))
    (:`NewEnumerator1`
      (`AudioComponent.FadeOut` (`self.Idle Sound Component`) 0.5 0.0 "Linear")
      (bind _returnvalue_2 (`GameplayStatics.SpawnSoundAttached` (`self.Movement Sound`) (`Actor.RootComponent` (`self.GetOwner`)) "None" (0.0 0.0 0.0) (struct) "KeepRelativeOffset" false 1.0 1.0 0.0 "/Game/Audio/SoundAttenuators/SA_EnemyTankMovement.SA_EnemyTankMovement" null))
      (bind _output_get_2 (set `self.Moving Sound Component` _returnvalue_2))
      (`AudioComponent.FadeIn` _output_get_2 0.5 1.0 0.0 "Linear")
      (`KismetSystemLibrary.PrintString` "Moving Sound State"))))

(fn `Play Current Player  Movement State Sound`
  (switch `/Game/Player/FSM/EMovementMode` (`/Game/Player/Pawns/BP_PlayerPawn.Current Movement Mode` (`self.As BP Player Pawn`))
    (:`NewEnumerator0`
      (`AudioComponent.FadeOut` (`self.Moving Sound Component`) 0.5 0.0 "Linear")
      (bind _returnvalue (`GameplayStatics.SpawnSoundAttached` (`self.Idle Sound`) (`Actor.RootComponent` (`self.GetOwner`)) "None" (0.0 0.0 0.0) (struct) "KeepRelativeOffset" false 1.0 1.0 0.0 null null))
      (bind _output_get (set `self.Idle Sound Component` _returnvalue))
      (`AudioComponent.FadeIn` _output_get 0.5 1.0 0.0 "Linear")
      (`KismetSystemLibrary.PrintString` "IDLE SOUND STATE"))
    (:`NewEnumerator1`
      (`AudioComponent.FadeOut` (`self.Idle Sound Component`) 0.5 0.0 "Linear")
      (bind _returnvalue_2 (`GameplayStatics.SpawnSoundAttached` (`self.Movement Sound`) (`Actor.RootComponent` (`self.GetOwner`)) "None" (0.0 0.0 0.0) (struct) "KeepRelativeOffset" false 1.0 1.0 0.0 null null))
      (bind _output_get_2 (set `self.Moving Sound Component` _returnvalue_2))
      (`AudioComponent.FadeIn` _output_get_2 0.5 1.0 0.0 "Linear")
      (`KismetSystemLibrary.PrintString` "Moving Sound State"))))

(fn `Play Death Sound`
  (if (== (`self.GetOwner`) (`GameplayStatics.GetPlayerPawn` 0))
    (`/Engine/EditorBlueprintResources/StandardMacros.IsValid` (`self.Death Sound`)
      (:`Is Valid`
        (`GameplayStatics.PlaySound2D` (`self.Death Sound`) 1.0 1.0 0.0 null null))
      (:`Is Not Valid`
        (`KismetSystemLibrary.PrintString` "Death sound is not valid or null")))
    (else
      (`/Engine/EditorBlueprintResources/StandardMacros.IsValid` (`self.Death Sound`)
        (:`Is Valid`
          (`GameplayStatics.PlaySound2D` (`self.Death Sound`) 1.0 1.0 0.0 null null))
        (:`Is Not Valid`
          (`KismetSystemLibrary.PrintString` "Death sound is not valid or null"))))))