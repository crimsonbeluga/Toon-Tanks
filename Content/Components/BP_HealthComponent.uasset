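; BP_HealthComponent tracks its owner's health, starting at the maximum and broadcasting changes through OnHealthChanged.
; ApplyDamage fires a damage delegate on every call, subtracts only while health is positive, and calls HandleDeath on the owner's BP_DeathComponent when health reaches zero or below.
; AddHealth raises health up to a hardcoded cap of 100, independent of the max health variable, then broadcasts the new value.
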(event `self.ReceiveBeginPlay`
  (bind _output_get (set `self.Current Health` (`self.Max Heath`)))
  (`self.OnHealthChanged` _output_get (`self.Max Heath`)))

(fn `Add Health`
  (params (`Added Health` :type "Float (double-precision)"))
  (bind _returnvalue (+ (`self.Current Health`) `Added Health`))
  (if (>= _returnvalue 100.0)
    (set `self.Current Health` 100.0)
    (`self.OnHealthChanged` (`self.Current Health`) (`self.Max Heath`))
    (else
      (set `self.Current Health` _returnvalue)
      (`self.OnHealthChanged` (`self.Current Health`) (`self.Max Heath`)))))

(fn `ApplyDamage`
  (params (`Damage Amount` :type "Float (double-precision)"))
  (locals (`Local Damage Amount` :type "Float (double-precision)"))
  (bind _returnvalue (`self.GetOwner`))
  (set `local.Local Damage Amount` `Damage Amount`)
  (`self.Apply Damage Delegate`)
  (if (<= (`self.Current Health`) 0.0)
    (`KismetSystemLibrary.PrintString` "Pawn is Dead Health is: 0" false false)
    (else
      (bind _output_get (set `self.Current Health` (- (`self.Current Health`) (`local.Local Damage Amount`))))
      (`self.OnHealthChanged` _output_get (`self.Max Heath`))
      (if (<= (`self.Current Health`) 0.0)
        (`/Game/Components/BP_DeathComponent.Handle Death` (`Actor.GetComponentByClass` _returnvalue "/Game/Components/BP_DeathComponent.BP_DeathComponent_C") _returnvalue)
        (`KismetSystemLibrary.PrintString` "BP_HealthComponent - Apply Damage: Handle Death Called" false false)))))