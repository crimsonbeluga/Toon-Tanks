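; BP_BaseEnemyPawn is a base enemy pawn that provides an AimAtTarget function for turning its AimPivot toward the first player's pawn.
; AimAtTarget interpolates the pivot's world yaw toward a look-at rotation at RotationSpeed, keeping the actor's own pitch and roll.
; It caps delta time at roughly one 60 fps frame, limiting the turn step during long frames.
; The event graph and construction script are empty, and nothing here calls AimAtTarget.
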(event `self.ReceiveTick`
  (params (DeltaSeconds :type "Float (single-precision)")))

(fn `Aim At Target`
  (params (`Delta Time` :type "Float (double-precision)"))
  (locals (`Player Location` :type "Vector Structure" :default (0.0 0.0 0.0)) (`Desired Rotation` :type "Rotator Structure") (`Effective Delta ` :type "Float (double-precision)"))
  (bind (_returnvalue_roll _returnvalue_pitch) (`KismetMathLibrary.BreakRotator` (`self.K2_GetActorRotation`)))
  (bind (_returnvalue_roll_2 _returnvalue_pitch_2 _returnvalue_yaw) (`KismetMathLibrary.BreakRotator` (`SceneComponent.K2_GetComponentRotation` (`self.Aim Pivot`))))
  (bind (_returnvalue_roll_3 _returnvalue_pitch_3 _returnvalue_yaw_2) (`KismetMathLibrary.BreakRotator` (`KismetMathLibrary.FindLookAtRotation` (`SceneComponent.K2_GetComponentLocation` (`self.Aim Pivot`)) (`local.Player Location`))))
  (bind (_returnvalue_roll_4 _returnvalue_pitch_4 _returnvalue_yaw_3) (`KismetMathLibrary.BreakRotator` (`KismetMathLibrary.RInterpTo` (`KismetMathLibrary.MakeRotator` 0.0 0.0 _returnvalue_yaw) (`KismetMathLibrary.MakeRotator` 0.0 0.0 _returnvalue_yaw_2) (`local.Effective Delta `) (`self.Rotation Speed`))))
  (set `local.Effective Delta ` (`KismetMathLibrary.FMin` `Delta Time` 0.016))
  (set `local.Player Location` (`self.K2_GetActorLocation` (`GameplayStatics.GetPlayerPawn` 0)))
  (bind _output_get (set `local.Desired Rotation` (`KismetMathLibrary.MakeRotator` _returnvalue_roll _returnvalue_pitch _returnvalue_yaw_3)))
  (`SceneComponent.K2_SetWorldRotation` (`self.Aim Pivot`) _output_get false false)
  (`KismetSystemLibrary.PrintString` "Aiming AT target" false false))

(fn `UserConstructionScript`)