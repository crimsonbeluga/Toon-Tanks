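; BP_BaseEnemyController is an enemy AI controller that uses perception to track the player in the Blackboard.
; Perception updates feed HandleSightConfiguration, which stores the player pawn under the player key when a successful sight stimulus comes from it.
; Any unsuccessful stimulus, regardless of actor or sense, clears that key and prints a debug message.
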(event `self.ReceiveBeginPlay`)

(event `self.AIPerception.OnTargetPerceptionUpdated`
  (params (Actor :type "Actor Object Reference") (Stimulus :type "AIStimulus Structure"))
  (`self.Handle Sight Configuration` Actor Stimulus))

(fn `Handle Sight Configuration`
  (params (A :type "Object Object Reference") (Stimulus :type "AIStimulus Structure"))
  (bind _returnvalue (`GameplayStatics.GetPlayerPawn` 0))
  (bind _output_get (set `self.Stimulus` Stimulus))
  (if (`.bSuccessfullySensed` (break `AIStimulus` _output_get))
    (bind _returnvalue_2 (`AIPerceptionSystem.GetSenseClassForStimulus` (`self.Stimulus`)))
    (if (== _returnvalue_2 "/Script/AIModule.AISense_Sight")
      (if (== A _returnvalue)
        (set `self.Seen Actor` _returnvalue)
        (`BlackboardComponent.SetValueAsObject` (`AIBlueprintHelperLibrary.GetBlackboard` null) (`self.BBKN Player`) (`self.Seen Actor`))))
    (else
      (`BlackboardComponent.SetValueAsObject` (`AIBlueprintHelperLibrary.GetBlackboard` null) (`self.BBKN Player`) null)
      (`KismetSystemLibrary.PrintString` "BP_BaseEnemyController - Handle Sight Configuration: Black Board value of player cleared"))))

(fn `UserConstructionScript`)