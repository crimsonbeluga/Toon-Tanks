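; BP_TrailVFXActor is an actor that carries a trail effect, using either a Niagara or a Cascade particle system.
; HandleSpawningVFX attaches the Niagara system to the root if it is valid, otherwise falls back to the particle system, and stores the spawned component.
; HandleDisipatingVFX deactivates both emitter references, then waits before destroying the actor, leaving time for the trail to fade.
; Nothing runs on BeginPlay or Tick.
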(event `self.ReceiveBeginPlay`)

(event `Handle Disipating VFX`
  (`self.Deactivate VFX`)
  (`KismetSystemLibrary.Delay` 10.0)
  (`self.K2_DestroyActor`))

(fn `Deactivate VFX`
  (`ActorComponent.Deactivate` (`self.Particle Emitter`))
  (`ActorComponent.Deactivate` (`self.NIagara Emiiter`)))

(fn `Handle Spawning VFX`
  (`/Engine/EditorBlueprintResources/StandardMacros.IsValid` (`self.Niagara System`)
    (:`Is Valid`
      (bind _returnvalue (`NiagaraFunctionLibrary.SpawnSystemAttached` (`self.Niagara System`) (`self.DefaultSceneRoot`) "None" (0.0 0.0 0.0) (struct) "KeepRelativeOffset"))
      (bind _output_get (set `self.NIagara Emiiter` _returnvalue))
      (`KismetSystemLibrary.PrintString` (`KismetStringLibrary.Concat_StrStr` "BP_Trail  VFX Actor - Handle Spawning VFX: Spawned VFx System Name:" (`KismetSystemLibrary.GetDisplayName` _output_get)) false false))
    (:`Is Not Valid`
      (`/Engine/EditorBlueprintResources/StandardMacros.IsValid` (`self.Particle System`)
        (:`Is Valid`
          (bind _returnvalue_2 (`GameplayStatics.SpawnEmitterAttached` (`self.Particle System`) (`self.DefaultSceneRoot`)))
          (bind _output_get_2 (set `self.Particle Emitter` _returnvalue_2))
          (`KismetSystemLibrary.PrintString` (`KismetStringLibrary.Concat_StrStr` "BP_Trail  VFX Actor - Handle Spawning VFX: Spawned VFx System Name:" (`KismetSystemLibrary.GetDisplayName` _output_get_2)) false false))
        (:`Is Not Valid`
          (`KismetSystemLibrary.PrintString` "BP_TrailVFXActor - Handle Spawning VFX: neither the niagara system or the particle system is valud"))))))

(fn `UserConstructionScript`)