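; Toon Tanks game mode that snapshots the level at BeginPlay and provides a world reset for the player, enemies and weapon pickups.
; It stores the first PlayerStart transform as the checkpoint, replaceable via SetPlayerSpawnTransform, plus struct arrays of each enemy's and pickup's class, transform and reference.
; HandleWorldReset recreates the player at the checkpoint, teleports surviving actors back and respawns missing ones, restoring enemy patrol paths on respawn.
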(event `self.ReceiveBeginPlay`
  (`self.Handle World Start`))

(fn `Handle Respawning Enemies`
  (locals (`Current Enemy` :type "/Game/AI/Pawns/BP_BaseEnemyPawn Object Reference") (`Enemy Class` :type "/Game/AI/Pawns/BP_BaseEnemyPawn Class Reference") (`Start Transform` :type "Transform Structure") (`Array Index` :type Integer) (`Patrol Points` :type "Map of /Game/AI/PatrolPoints/BP_PatrolPointMarkers Object Reference to Float (double-precision)"))
  (for (_array_element _array_index) (`self.EnemySpawnDataArray`)
    (set `local.Enemy Class` (break `/Game/Core/GameModes/Structs/S_EnemySpawnData` _array_element))
    (set `local.Start Transform` (`.StartTransform_7_D51EF64847E27ECBA62628A5BB0E5279` (break `/Game/Core/GameModes/Structs/S_EnemySpawnData` _array_element)))
    (set `local.Current Enemy` (`.CurrentEnemy_9_DAA3F27E4136C66324412188CC3FFD37` (break `/Game/Core/GameModes/Structs/S_EnemySpawnData` _array_element)))
    (set `local.Patrol Points` (`.PatrolPoints_19_FBF3673C42E7F22DE937DF9344DCA6F5` (break `/Game/Core/GameModes/Structs/S_EnemySpawnData` _array_element)))
    (set `local.Array Index` _array_index)
    (`/Engine/EditorBlueprintResources/StandardMacros.IsValid` (`local.Current Enemy`)
      (:`Is Valid`
        (`self.K2_SetActorTransform` (`local.Current Enemy`) (`local.Start Transform`) false true))
      (:`Is Not Valid`
        (bind _returnvalue (`|SpawnActorFromClass` (`local.Enemy Class`) (`local.Start Transform`) "AlwaysSpawn" "MultiplyWithRoot" null null))
        (bind _output_get (set `local.Current Enemy` _returnvalue))
        (`KismetArrayLibrary.Array_Set` (`self.EnemySpawnDataArray`) (`local.Array Index`) (make `/Game/Core/GameModes/Structs/S_EnemySpawnData` (`local.Enemy Class`) (`local.Start Transform`) _output_get (`local.Patrol Points`)))
        (set `/Game/AI/Components/AI_PathFollowingComponent.Patrol Path` (`local.Patrol Points`) (`/Game/AI/Pawns/BP_BaseEnemyPawn.AI_PathFollowingComponent` (`local.Current Enemy`)))))))

(fn `Handle Respawning Pickups`
  (locals (`Pickup Class` :type "/Game/Environment/Pickups/WeaponPickups/BP_WeaponClassPickUpBase Class Reference") (`Start Transform` :type "Transform Structure") (`Current Pickup` :type "/Game/Environment/Pickups/WeaponPickups/BP_WeaponClassPickUpBase Object Reference") (`Array Index` :type Integer))
  (for (_array_element _array_index) (`self.PickUpDataArray`)
    (set `local.Pickup Class` (break `/Game/Core/GameModes/Structs/S_PickUpSpawnData` _array_element))
    (set `local.Start Transform` (`.StartTransform_7_D51EF64847E27ECBA62628A5BB0E5279` (break `/Game/Core/GameModes/Structs/S_PickUpSpawnData` _array_element)))
    (set `local.Current Pickup` (`.CurrentPickup_13_DAA3F27E4136C66324412188CC3FFD37` (break `/Game/Core/GameModes/Structs/S_PickUpSpawnData` _array_element)))
    (set `local.Array Index` _array_index)
    (`/Engine/EditorBlueprintResources/StandardMacros.IsValid` (`local.Current Pickup`)
      (:`Is Valid`
        (`self.K2_SetActorTransform` (`local.Current Pickup`) (`local.Start Transform`) false true))
      (:`Is Not Valid`
        (bind _returnvalue (`|SpawnActorFromClass` (`local.Pickup Class`) (`local.Start Transform`) "Undefined" "MultiplyWithRoot" null null))
        (`KismetArrayLibrary.Array_Set` (`self.PickUpDataArray`) (`local.Array Index`) (make `/Game/Core/GameModes/Structs/S_PickUpSpawnData` (`local.Pickup Class`) (`local.Start Transform`) _returnvalue))))))

(fn `Handle Respawning Player`
  (`self.K2_DestroyActor` (`GameplayStatics.GetPlayerPawn` 0))
  (`self.RestartPlayerAtTransform` (`GameplayStatics.GetPlayerController` 0) (`self.Player Checkpoint Spawn Transform`))
  (`KismetSystemLibrary.PrintString` "New Player spawned" false false))

(fn `Handle World Reset`
  (`self.Handle Respawning Player`)
  (`self.Handle Respawning Enemies`)
  (`self.Handle Respawning Pickups`))

(fn `Handle World Start`
  (`self.Set Player Start Transform`)
  (`self.Store Enemies Start Position`)
  (`self.Store Pick Up Start Positions`))

(fn `Set  Player Spawn Transform`
  (params (`New Spawn Transform` :type "Transform Structure"))
  (set `self.Player Checkpoint Spawn Transform` `New Spawn Transform`)
  (`KismetSystemLibrary.PrintString` "BP_ToonTanksGameMode - Set Spawn Transform: New Spawn Transform Set" false false (struct :`G` 0.66 :`B` 1.0 :`A` 1.0) 5.0))

(fn `Set Player Start Transform`
  (bind _outactors (`GameplayStatics.GetAllActorsOfClass` "/Script/Engine.PlayerStart"))
  (set `self.Player Checkpoint Spawn Transform` (`self.GetTransform` (`|GetArrayItem` _outactors))))

(fn `Store Enemies Start Position`
  (locals (`Array Element` :type "/Game/AI/Pawns/BP_BaseEnemyPawn Object Reference"))
  (bind _outactors (`GameplayStatics.GetAllActorsOfClass` "/Game/AI/Pawns/BP_BaseEnemyPawn.BP_BaseEnemyPawn_C"))
  (for _array_element _outactors
    (set `local.Array Element` _array_element)
    (`KismetArrayLibrary.Array_Add` (`self.EnemySpawnDataArray`) (make `/Game/Core/GameModes/Structs/S_EnemySpawnData` (`GameplayStatics.GetObjectClass` (`local.Array Element`)) (`self.GetTransform` (`local.Array Element`)) (`local.Array Element`) (`/Game/AI/Components/AI_PathFollowingComponent.Patrol Path` (`/Game/AI/Pawns/BP_BaseEnemyPawn.AI_PathFollowingComponent` (`local.Array Element`)))))))

(fn `Store Pick Up Start Positions`
  (locals (`Array Element` :type "/Game/Environment/Pickups/WeaponPickups/BP_WeaponClassPickUpBase Object Reference"))
  (bind _outactors (`GameplayStatics.GetAllActorsOfClass` "/Game/Environment/Pickups/WeaponPickups/BP_WeaponClassPickUpBase.BP_WeaponClassPickUpBase_C"))
  (for _array_element _outactors
    (set `local.Array Element` _array_element)
    (`KismetArrayLibrary.Array_Add` (`self.PickUpDataArray`) (make `/Game/Core/GameModes/Structs/S_PickUpSpawnData` (`GameplayStatics.GetObjectClass` (`local.Array Element`)) (`self.GetTransform` (`local.Array Element`)) (`local.Array Element`)))))

(fn `UserConstructionScript`)