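; Base teleporter actor that moves the player pawn to a linked destination actor when the pawn enters its box trigger.
; On overlap, if it is not on cooldown, it flags the destination as cooling down and sets the pawn's transform to that actor's location and rotation.
; Leaving a box clears that teleporter's cooldown, which stops linked pairs from bouncing the player straight back.
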(event `self.Box.OnComponentBeginOverlap`
  (params (OverlappedComponent :type "PrimitiveComponent Object Reference") (OtherActor :type "Actor Object Reference") (OtherComp :type "PrimitiveComponent Object Reference") (OtherBodyIndex :type Integer) (bFromSweep :type Boolean) (SweepResult :type "HitResult Structure (by ref)"))
  (if (== OtherActor (`GameplayStatics.GetPlayerPawn` 0))
    (`/Engine/EditorBlueprintResources/StandardMacros.IsValid` (`self.Teleport Location Actor`)
      (:`Is Valid`
        (if (not (`self.bIsOnCoolDown`))
          (set `/Game/Environment/Teleporter/BP_BaseTeleporter.bIsOnCoolDown` true (`self.Teleport Location Actor`))
          (`self.Handle Teleport `))))))

(event `self.Box.OnComponentEndOverlap`
  (params (OverlappedComponent :type "PrimitiveComponent Object Reference") (OtherActor :type "Actor Object Reference") (OtherComp :type "PrimitiveComponent Object Reference") (OtherBodyIndex :type Integer))
  (set `self.bIsOnCoolDown` false))

(fn `Handle Teleport `
  (`self.K2_SetActorTransform` (`GameplayStatics.GetPlayerPawn` 0) (`KismetMathLibrary.MakeTransform` (`self.K2_GetActorLocation` (`self.Teleport Location Actor`)) (`self.K2_GetActorRotation` (`self.Teleport Location Actor`))) false false))

(fn `UserConstructionScript`)