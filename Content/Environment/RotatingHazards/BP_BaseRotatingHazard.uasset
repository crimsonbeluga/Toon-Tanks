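; Base Blueprint for rotating hazards that spins the actor around yaw every Tick at RotationSpeed, scaled by delta time.
; It provides two handlers for player pawn 0: one applies DamageAmount through BP_HealthComponent, the other calls HandleDeath on BP_DeathComponent.
; Neither handler is called in this Blueprint, and its overlap event is empty.
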(event `self.ReceiveActorBeginOverlap`
  (params (OtherActor :type "Actor Object Reference")))

(event `self.ReceiveTick`
  (params (DeltaSeconds :type "Float (single-precision)"))
  (`self.Handle Rotation` DeltaSeconds))

(fn `Handle Dealing  Damage`
  (params (`Other Actor` :type "Object Object Reference"))
  (bind _returnvalue (`GameplayStatics.GetPlayerPawn` 0))
  (if (== `Other Actor` _returnvalue)
    (`/Game/Components/BP_HealthComponent.ApplyDamage` (`self.GetComponentByClass` _returnvalue "/Game/Components/BP_HealthComponent.BP_HealthComponent_C") (`self.Damage Amount`))))

(fn `Handle Dealing Death`
  (params (`Other Actor` :type "Object Object Reference"))
  (bind _returnvalue (`GameplayStatics.GetPlayerPawn` 0))
  (if (== `Other Actor` _returnvalue)
    (`/Game/Components/BP_DeathComponent.Handle Death` (`self.GetComponentByClass` _returnvalue "/Game/Components/BP_DeathComponent.BP_DeathComponent_C") _returnvalue)))

(fn `Handle Rotation`
  (params (`Input Delta Time` :type "Float (double-precision)"))
  (locals (`Desired Rotation` :type "Rotator Structure") (`Dela Time` :type "Float (double-precision)"))
  (bind (_returnvalue_roll _returnvalue_pitch _returnvalue_yaw) (`KismetMathLibrary.BreakRotator` (`self.K2_GetActorRotation`)))
  (set `local.Dela Time` `Input Delta Time`)
  (bind _output_get (set `local.Desired Rotation` (`KismetMathLibrary.MakeRotator` _returnvalue_roll _returnvalue_pitch (+ (* (`self.Rotation Speed`) (`local.Dela Time`)) _returnvalue_yaw))))
  (`self.K2_SetActorRotation` _output_get))

(fn `UserConstructionScript`)