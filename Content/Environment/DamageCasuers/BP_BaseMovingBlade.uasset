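; Base moving-blade hazard that shuttles back and forth between two endpoints and kills the player on contact.
; Each tick it moves the Blade at constant speed toward the current endpoint component's relative location, flipping direction once within ReachTolerance.
; HitBox overlaps call the player pawn's death component, but only when the overlapping component is that pawn's own HitBox.
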(event `self.ReceiveTick`
  (params (DeltaSeconds :type "Float (single-precision)"))
  (if (`self.Moving To End Point Two`)
    (`self.Move To End Point Two` DeltaSeconds)
    (else
      (`self.Move To End Point One` DeltaSeconds))))

(event `self.Hit Box.OnComponentBeginOverlap`
  (params (OverlappedComponent :type "PrimitiveComponent Object Reference") (OtherActor :type "Actor Object Reference") (OtherComp :type "PrimitiveComponent Object Reference") (OtherBodyIndex :type Integer) (bFromSweep :type Boolean) (SweepResult :type "HitResult Structure (by ref)"))
  (`self.Handle Killing Player` OverlappedComponent OtherActor OtherComp))

(fn `Handle Killing Player`
  (params (`Input Overlapped Component` :type "PrimitiveComponent Object Reference") (`Input Other Actor` :type "Actor Object Reference") (`Input Other Comp` :type "PrimitiveComponent Object Reference"))
  (locals (`Local Overlapped Component` :type "PrimitiveComponent Object Reference") (`Local Other Actor` :type "Actor Object Reference") (`Local Other Comp` :type "PrimitiveComponent Object Reference") (`BP_PlayerPawn Ref` :type "/Game/Player/Pawns/BP_PlayerPawn Object Reference"))
  (bind _bp_deathcomponent (`/Game/Player/Pawns/BP_PlayerPawn.BP_DeathComponent` (`local.BP_PlayerPawn Ref`)))
  (set `local.Local Overlapped Component` `Input Overlapped Component`)
  (set `local.Local Other Actor` `Input Other Actor`)
  (set `local.Local Other Comp` `Input Other Comp`)
  (if (== (`local.Local Other Actor`) (`GameplayStatics.GetPlayerPawn` 0))
    (bind _asbp_player_pawn (cast `/Game/Player/Pawns/BP_PlayerPawn` (`GameplayStatics.GetPlayerPawn` 0))
      (:`then`
        (set `local.BP_PlayerPawn Ref` _asbp_player_pawn)
        (if (== (`local.Local Other Comp`) (`/Game/Player/Pawns/BP_PlayerPawn.Hit Box` (`local.BP_PlayerPawn Ref`)))
          (`/Engine/EditorBlueprintResources/StandardMacros.IsValid` _bp_deathcomponent
            (:`Is Valid`
              (`/Game/Components/BP_DeathComponent.Handle Death` _bp_deathcomponent (`local.BP_PlayerPawn Ref`)))
            (:`Is Not Valid`
              (`KismetSystemLibrary.PrintString` "BP_BaseMovingBlade - Handle Killing Player: Death Component on BP_PlayePawn is not valid")))))
      (:`CastFailed`
        (`KismetSystemLibrary.PrintString` "BP_BaseMovingBlade - Handle Killing Player: Cast to BP_PlayerPawn Failed")))))

(fn `Move To End Point One`
  (params (`Input Delta Time` :type "Float (double-precision)"))
  (locals (`Current Relative Location` :type "Vector Structure" :default (0.0 0.0 0.0)) (`Target Location` :type "Vector Structure" :default (0.0 0.0 0.0)) (`Local Delta Time` :type "Float (double-precision)"))
  (set `local.Local Delta Time` `Input Delta Time`)
  (set `local.Current Relative Location` (`SceneComponent.RelativeLocation` (`self.Blade`)))
  (set `local.Target Location` (`SceneComponent.RelativeLocation` (`self.End Point One`)))
  (`SceneComponent.K2_SetRelativeLocation` (`self.Blade`) (`KismetMathLibrary.VInterpTo_Constant` (`local.Current Relative Location`) (`local.Target Location`) (`local.Local Delta Time`) (`self.Movement Speed`)) false false)
  (if (== (`local.Current Relative Location`) (`local.Target Location`) :`ErrorTolerance` (`self.Reach Tolerance`))
    (set `self.Moving To End Point Two` true)))

(fn `Move To End Point Two`
  (params (`Input Delta Time` :type "Float (double-precision)"))
  (locals (`Current Relative Location` :type "Vector Structure" :default (0.0 0.0 0.0)) (`Target Location` :type "Vector Structure" :default (0.0 0.0 0.0)) (`Local Delta Time` :type "Float (double-precision)"))
  (set `local.Local Delta Time` `Input Delta Time`)
  (set `local.Current Relative Location` (`SceneComponent.RelativeLocation` (`self.Blade`)))
  (set `local.Target Location` (`SceneComponent.RelativeLocation` (`self.End Point Two`)))
  (`SceneComponent.K2_SetRelativeLocation` (`self.Blade`) (`KismetMathLibrary.VInterpTo_Constant` (`local.Current Relative Location`) (`local.Target Location`) (`local.Local Delta Time`) (`self.Movement Speed`)) false false)
  (if (== (`local.Current Relative Location`) (`local.Target Location`) :`ErrorTolerance` (`self.Reach Tolerance`))
    (set `self.Moving To End Point Two` false)))

(fn `UserConstructionScript`)