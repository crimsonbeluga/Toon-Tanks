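; BP_GroundExplosive is a one-shot environmental hazard that damages the player on contact.
; Its Box overlap responds only to the player 0 pawn, and only if that pawn has a BP_HealthComponent.
; It applies DamageAmount through that component, spawns both Niagara and Cascade effects with a hit sound at its location, then destroys itself.
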(event `self.ReceiveActorBeginOverlap`
  (params (OtherActor :type "Actor Object Reference")))

(event `self.Box.OnComponentBeginOverlap`
  (params (OverlappedComponent :type "PrimitiveComponent Object Reference") (OtherActor :type "Actor Object Reference") (OtherComp :type "PrimitiveComponent Object Reference") (OtherBodyIndex :type Integer) (bFromSweep :type Boolean) (SweepResult :type "HitResult Structure (by ref)"))
  (bind _returnvalue (`self.GetComponentByClass` (`self.Other Actor`) "/Game/Components/BP_HealthComponent.BP_HealthComponent_C"))
  (bind _output_get (set `self.Other Actor` OtherActor))
  (if (== _output_get (`GameplayStatics.GetPlayerPawn` 0))
    (`/Engine/EditorBlueprintResources/StandardMacros.IsValid` _returnvalue
      (:`Is Valid`
        (`/Game/Components/BP_HealthComponent.ApplyDamage` _returnvalue (`self.Damage Amount`))
        (`NiagaraFunctionLibrary.SpawnSystemAtLocation` (`self.Niagara VFX`) (`self.K2_GetActorLocation`))
        (`GameplayStatics.SpawnEmitterAtLocation` (`self.Cascade VFX`) (`self.K2_GetActorLocation`))
        (`GameplayStatics.PlaySoundAtLocation` (`self.Hit Sound`) (`self.K2_GetActorLocation`) (struct) 1.0 1.0 0.0 null null null null)
        (`self.K2_DestroyActor`)))))

(fn `UserConstructionScript`)