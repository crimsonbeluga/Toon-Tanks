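; Base moving platform actor that shuttles its platform mesh back and forth between a start point and an end point.
; On BeginPlay it caches the world locations of the start and end marker meshes.
; Each Tick moves the mesh at constant speed toward the current target with a swept VInterpToConstant move, flipping direction when within a reach tolerance.
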(event `self.ReceiveBeginPlay`
  (set `self.Platform  Location` (`SceneComponent.RelativeLocation` (`self.Platform Mesh`)))
  (set `self.Start Point Location` (`SceneComponent.K2_GetComponentLocation` (`self.Start Point Mesh`)))
  (set `self.End Point Location` (`SceneComponent.K2_GetComponentLocation` (`self.End Point Mesh`))))

(event `self.ReceiveTick`
  (params (DeltaSeconds :type "Float (single-precision)"))
  (if (`self.BIsMovingToEnd`)
    (`self.Move To End Point` DeltaSeconds)
    (else
      (`self.Move To Start Point` DeltaSeconds))))

(fn `Move To End Point`
  (params (`Delta Time` :type "Float (double-precision)"))
  (`SceneComponent.K2_SetWorldLocation` (`self.Platform Mesh`) (`KismetMathLibrary.VInterpTo_Constant` (`SceneComponent.K2_GetComponentLocation` (`self.Platform Mesh`)) (`self.End Point Location`) `Delta Time` (`self.Movement Speed`)) true false)
  (if (== (`SceneComponent.K2_GetComponentLocation` (`self.Platform Mesh`)) (`self.End Point Location`) :`ErrorTolerance` (`self.Reach Tolerance`))
    (set `self.BIsMovingToEnd` false)))

(fn `Move To Start Point`
  (params (`Delta Time` :type "Float (double-precision)"))
  (`SceneComponent.K2_SetWorldLocation` (`self.Platform Mesh`) (`KismetMathLibrary.VInterpTo_Constant` (`SceneComponent.K2_GetComponentLocation` (`self.Platform Mesh`)) (`self.Start Point Location`) `Delta Time` (`self.Movement Speed`)) true false)
  (if (== (`SceneComponent.K2_GetComponentLocation` (`self.Platform Mesh`)) (`self.Start Point Location`) :`ErrorTolerance` (`self.Reach Tolerance`))
    (set `self.BIsMovingToEnd` true)))

(fn `UserConstructionScript`)