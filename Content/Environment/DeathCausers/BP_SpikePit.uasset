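; BP_SpikePit is an environmental hazard that kills the player on contact.
; When its Box overlaps something, it checks that the actor is player 0's pawn and the touching component is that BP_PlayerPawn's HitBox.
; It then calls HandleDeath on the pawn's BPDeathComponent, so other parts of the pawn do not trigger death.
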(event `self.Box.OnComponentBeginOverlap`
  (params (OverlappedComponent :type "PrimitiveComponent Object Reference") (OtherActor :type "Actor Object Reference") (OtherComp :type "PrimitiveComponent Object Reference") (OtherBodyIndex :type Integer) (bFromSweep :type Boolean) (SweepResult :type "HitResult Structure (by ref)"))
  (set `self.Other Actor` OtherActor)
  (set `self.Other Comp` OtherComp)
  (if (== (`self.Other Actor`) (`GameplayStatics.GetPlayerPawn` 0))
    (bind _asbp_player_pawn (cast `/Game/Player/Pawns/BP_PlayerPawn` (`GameplayStatics.GetPlayerPawn` 0)))
    (if (== (`self.Other Comp`) (`/Game/Player/Pawns/BP_PlayerPawn.Hit Box` _asbp_player_pawn))
      (`/Game/Components/BP_DeathComponent.Handle Death` (`/Game/Player/Pawns/BP_PlayerPawn.BP_DeathComponent` _asbp_player_pawn) _asbp_player_pawn))))

(fn `UserConstructionScript`)