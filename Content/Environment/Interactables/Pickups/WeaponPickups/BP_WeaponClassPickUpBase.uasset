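; Base weapon pickup actor that gives the player a weapon when touched.
; Each tick it spins its rotating component around yaw at a configurable speed.
; When the player pawn overlaps the sphere, it passes its WeaponData to that pawn's BP_WeaponComponent to equip, plays a pickup sound and destroys itself.
; Other overlapping actors only trigger a debug print.
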(event `self.ReceiveTick`
  (params (DeltaSeconds :type "Float (single-precision)"))
  (`self.Rotate Mesh` DeltaSeconds))

(event `self.Sphere.OnComponentBeginOverlap`
  (params (OverlappedComponent :type "PrimitiveComponent Object Reference") (OtherActor :type "Actor Object Reference") (OtherComp :type "PrimitiveComponent Object Reference") (OtherBodyIndex :type Integer) (bFromSweep :type Boolean) (SweepResult :type "HitResult Structure (by ref)"))
  (if (== OtherActor (`GameplayStatics.GetPlayerPawn` 0))
    (bind _output_get (set `self.Player Pawn` OtherActor))
    (`/Game/Components/BP_WeaponComponent.Equip Weapon ` (`self.GetComponentByClass` _output_get "/Game/Components/BP_WeaponComponent.BP_WeaponComponent_C") (`self.Weapon Data`))
    (`GameplayStatics.PlaySound2D` "/Game/Audio/AudioClips/SFX/Pickup_Weapon_Sound_Effect.Pickup_Weapon_Sound_Effect" 1.0 1.0 0.0 null null)
    (`self.K2_DestroyActor`)
    (else
      (`KismetSystemLibrary.PrintString` "Overlapping actor was not the player pawn "))))

(fn `Rotate Mesh`
  (params (`Delta Seconds` :type "Float (double-precision)"))
  (locals (`Desired Rotation` :type "Rotator Structure" :default (struct)) (`Yaw Delta` :type "Float (double-precision)") (`Delta Rotation` :type "Rotator Structure" :default (struct)))
  (set `local.Yaw Delta` (* `Delta Seconds` (`self.Item Rotation Speed`)))
  (set `local.Delta Rotation` (`KismetMathLibrary.MakeRotator` 0.0 0.0 (`local.Yaw Delta`)))
  (`SceneComponent.K2_AddLocalRotation` (`self.Rotating Component`) (`local.Delta Rotation`) false false))

(fn `UserConstructionScript`)