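; BP_BaseHealthPickup is a base pickup that restores health to the player and then removes itself from the world.
; When its Box component is overlapped, it checks that the other actor is the first player's BP_PlayerPawn and the touched component is that pawn's HitBox.
; A valid overlap passes AddedHealthAmount to the pawn's BPHealthComponent through AddHealth, then destroys the pickup.
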(event `self.Box.OnComponentBeginOverlap`
  (params (OverlappedComponent :type "PrimitiveComponent Object Reference") (OtherActor :type "Actor Object Reference") (OtherComp :type "PrimitiveComponent Object Reference") (OtherBodyIndex :type Integer) (bFromSweep :type Boolean) (SweepResult :type "HitResult Structure (by ref)"))
  (bind _returnvalue (`GameplayStatics.GetPlayerPawn` 0))
  (set `self.Overlapped Component` OverlappedComponent)
  (set `self.Other Actor` OtherActor)
  (set `self.Other Comp` OtherComp)
  (if (== (`self.Other Actor`) _returnvalue)
    (bind _asbp_player_pawn (cast `/Game/Player/Pawns/BP_PlayerPawn` _returnvalue))
    (set `self.As BP Player Pawn` _asbp_player_pawn)
    (if (== (`/Game/Player/Pawns/BP_PlayerPawn.Hit Box` (`self.As BP Player Pawn`)) (`self.Other Comp`))
      (`/Game/Components/BP_HealthComponent.Add Health` (`/Game/Player/Pawns/BP_PlayerPawn.BP_HealthComponent` (`self.As BP Player Pawn`)) (`self.Added Health Amount`))
      (`self.K2_DestroyActor`))))

(fn `UserConstructionScript`)