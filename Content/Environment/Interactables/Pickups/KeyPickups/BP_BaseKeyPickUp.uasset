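; BP_BaseKeyPickUp is a base key pickup that an interactor collects into its inventory.
; On BeginPlay it attaches its Widget component to the Key component.
; Interact looks for a BP_InventoryComponent on the interactor and, if found, adds KeyData, plays a 2D pickup sound and destroys itself.
; A yaw-spin node remains in the graph but never runs.
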(event `self.ReceiveBeginPlay`
  (`SceneComponent.K2_AttachToComponent` (`self.Widget`) (`self.Key`) "None" "KeepRelative" "KeepRelative" "KeepRelative" true))

(event `self.ReceiveTick`
  (params (DeltaSeconds :type "Float (single-precision)")))

(event `/Game/Core/Interfaces/BPI_Interactable.Interact`
  (params (Interactor :type "Actor Object Reference"))
  (bind _returnvalue (`self.GetComponentByClass` Interactor "/Game/Components/BP_InventoryComponent.BP_InventoryComponent_C"))
  (`/Engine/EditorBlueprintResources/StandardMacros.IsValid` _returnvalue
    (:`Is Valid`
      (`/Game/Components/BP_InventoryComponent.Add Key` _returnvalue (`self.Key Data`))
      (`GameplayStatics.PlaySound2D` "/Game/Audio/AudioClips/SFX/SW_PickUpKeySound.SW_PickUpKeySound" 1.0 1.0 0.0 null null)
      (`self.K2_DestroyActor`))))

(fn `UserConstructionScript`)