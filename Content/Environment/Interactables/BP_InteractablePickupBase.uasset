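; BP_InteractablePickupBase is a base Blueprint for interactable pickups that carry an interaction prompt widget.
; Show and hide functions toggle the widget's visibility, with showing gated by a CanShowUI flag.
; The Interact event only prints a debug message and clears that flag, blocking later show calls without hiding a widget that is already visible.
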(event `/Game/Core/Interfaces/BPI_Interactable.Interact`
  (params (Interactor :type "Actor Object Reference"))
  (`KismetSystemLibrary.PrintString` "Interact on pick up base called")
  (`self.Set Show UI False`))

(fn `Hide Interact UI`
  (`SceneComponent.SetVisibility` (`self.Widget`) false false))

(fn `Set Show UI False`
  (set `self.bCanShowUI` false))

(fn `Show Interact UI`
  (if (`self.bCanShowUI`)
    (`SceneComponent.SetVisibility` (`self.Widget`) true false)))

(fn `UserConstructionScript`)