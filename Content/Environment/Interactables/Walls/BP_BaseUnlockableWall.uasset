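; Base interactable wall that unlocks when the interactor's inventory holds a key matching the wall's key type.
; Interact compares each key in the interactor's BP_InventoryComponent against KeyData, calling UnlockWall on a match and printing a message otherwise.
; UnlockWall runs once as a short cutscene: it removes input and the widget, blends the camera to the wall, plays a sound, disables glass collision, turns hieroglyphs green, then restores view and input.
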(event `Unlock Wall`
  (bind _returnvalue (`GameplayStatics.GetPlayerController` 0))
  (`/Engine/EditorBlueprintResources/StandardMacros.DoOnce` false
    (:`Completed`
      (`ActorComponent.K2_DestroyComponent` (`self.Widget`))
      (bind _asbp_player_controller (cast `/Game/Player/Controllers/BP_PlayerController` (`GameplayStatics.GetPlayerController` 0)))
      (`/Game/Player/Controllers/BP_PlayerController.Remove Input Mapping` _asbp_player_controller)
      (`PlayerController.SetViewTargetWithBlend` (`GameplayStatics.GetPlayerController` 0) self 0.0 "VTBlend_Linear" 0.0 false)
      (`GameplayStatics.PlaySound2D` "/Game/Audio/AudioClips/SFX/SW_UnlockGateSoundEffect.SW_UnlockGateSoundEffect" 1.0 1.0 0.0 null null)
      (`KismetSystemLibrary.Delay` 1.0)
      (`PrimitiveComponent.SetCollisionEnabled` (`self.Glass`) "NoCollision")
      (`PrimitiveComponent.SetMaterial` (`self.Hieroglyph Mesh Front`) 0 "/Game/Art/Materials/M_EmissiveGreen_Inst.M_EmissiveGreen_Inst")
      (`PrimitiveComponent.SetMaterial` (`self.Hieroglyph Mesh Back`) 0 "/Game/Art/Materials/M_EmissiveGreen_Inst.M_EmissiveGreen_Inst")
      (`KismetSystemLibrary.Delay` 1.0)
      (`PlayerController.SetViewTargetWithBlend` _returnvalue (`Controller.K2_GetPawn` _returnvalue) 0.0 "VTBlend_Linear" 0.0 false)
      (bind _asbp_player_controller_2 (cast `/Game/Player/Controllers/BP_PlayerController` (`GameplayStatics.GetPlayerController` 0)))
      (`/Game/Player/Controllers/BP_PlayerController.SetupDefaultInputMapping` _asbp_player_controller_2))))

(fn `Compare Key Values`
  (params (Interactor :type "Actor Object Reference"))
  (for _array_element (`/Game/Components/BP_InventoryComponent.List of Keys` (`self.GetComponentByClass` Interactor "/Game/Components/BP_InventoryComponent.BP_InventoryComponent_C"))
    (if (`|EnumEquality` (`/Game/Player/Inventory/Keys/PDA_Keys.Key Enum` _array_element) (`/Game/Player/Inventory/Keys/PDA_Keys.Key Enum` (`self.Key Data`)))
      (`self.Unlock Wall`)
      (else
        (`KismetSystemLibrary.PrintString` "Incorrect  key type") ; Handle incorrect key type here
      ))))

(fn `Interact`
  (params (Interactor :type "Actor Object Reference"))
  (`self.Compare Key Values` Interactor)
  (return))

(fn `UserConstructionScript`)