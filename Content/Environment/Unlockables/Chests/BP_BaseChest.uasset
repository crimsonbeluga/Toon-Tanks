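; Base chest Blueprint for unlockable chests that opens and ejects a key pickup when interacted with.
; Interact snaps the lid open by setting its world roll directly, then spawns the configured key pickup class at the loot spawn point.
; The pickup's mesh receives an unscaled impulse along the chest base's forward vector.
; No open state is tracked, so each interaction spawns another pickup.
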(event `/Game/Core/Interfaces/BPI_Interactable.Interact`
  (params (Interactor :type "Actor Object Reference"))
  (`self.Open Chest Lid`)
  (bind _returnvalue (`|SpawnActorFromClass` (`self.Key Pick Up Type`) (`SceneComponent.K2_GetComponentToWorld` (`self.Loot Spawn Point`)) "Undefined" "MultiplyWithRoot" null null))
  (`PrimitiveComponent.AddImpulse` (`/Game/Environment/KeyPickups/BP_BaseKeyPickUp.StaticMesh` _returnvalue) (`SceneComponent.GetForwardVector` (`self.Chest Base`)) "None" false))

(fn `Open Chest Lid`
  (bind (_returnvalue_roll _returnvalue_pitch _returnvalue_yaw) (`KismetMathLibrary.BreakRotator` (`SceneComponent.K2_GetComponentRotation` (`self.Chest Lid`))))
  (`SceneComponent.K2_SetWorldRotation` (`self.Chest Lid`) (`KismetMathLibrary.MakeRotator` -60.0 _returnvalue_pitch _returnvalue_yaw) false false))

(fn `UserConstructionScript`)