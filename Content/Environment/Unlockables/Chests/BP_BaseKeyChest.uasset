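; Base key chest that opens once on Interact and ejects a key pickup.
; Opening snaps the lid's roll, stops the chest's audio component and plays an open sound.
; It then spawns KeyPickUpType at LootSpawnPoint and launches its physics-simulated Key with randomized forward, upward and sideways impulses.
; A debug sphere is drawn around the spawn point in the construction script and every Tick.
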(event `self.ReceiveBeginPlay`)

(event `self.ReceiveTick`
  (params (DeltaSeconds :type "Float (single-precision)"))
  (`KismetSystemLibrary.DrawDebugSphere` (`SceneComponent.K2_GetComponentLocation` (`self.Loot Spawn Point`)) 550.0 12 (struct :`R` 1.0 :`G` 1.0 :`B` 1.0 :`A` 1.0) 0.0 2.0))

(event `/Game/Core/Interfaces/BPI_Interactable.Interact`
  (params (Interactor :type "Actor Object Reference"))
  (`/Engine/EditorBlueprintResources/StandardMacros.DoOnce` false
    (:`Completed`
      (`self.Open Chest Lid`)
      (bind _returnvalue (`|SpawnActorFromClass` (`self.Key Pick Up Type`) (`SceneComponent.K2_GetComponentToWorld` (`self.Loot Spawn Point`)) "AlwaysSpawn" "MultiplyWithRoot" null null))
      (bind _asbp_base_key_pick_up (cast `/Game/Environment/Pickups/KeyPickups/BP_BaseKeyPickUp` _returnvalue))
      (bind _key (`/Game/Environment/Pickups/KeyPickups/BP_BaseKeyPickUp.Key` _asbp_base_key_pick_up))
      (`PrimitiveComponent.SetSimulatePhysics` _key true)
      (`PrimitiveComponent.AddImpulse` _key (+ (* (`SceneComponent.GetForwardVector` (`self.Loot Spawn Point`)) (`KismetMathLibrary.RandomFloatInRange` (`self.Forward Impulse Min`) (`self.Forward Impulse Max`))) (* (`SceneComponent.GetUpVector` (`self.Loot Spawn Point`)) (`KismetMathLibrary.RandomFloatInRange` (`self.Upward Impulse Min`) (`self.Upward Impulse Max`))) (* (`SceneComponent.GetRightVector` (`self.Loot Spawn Point`)) (`KismetMathLibrary.RandomFloatInRange` (`self.Right Impulse Min`) (`self.Right Impulse Max`)))) "None" true))))

(fn `Open Chest Lid`
  (bind (_returnvalue_roll _returnvalue_pitch _returnvalue_yaw) (`KismetMathLibrary.BreakRotator` (`SceneComponent.K2_GetComponentRotation` (`self.Chest Lid`))))
  (`SceneComponent.K2_SetWorldRotation` (`self.Chest Lid`) (`KismetMathLibrary.MakeRotator` -60.0 _returnvalue_pitch _returnvalue_yaw) false false)
  (`AudioComponent.Stop` (`self.Audio`))
  (`/Engine/EditorBlueprintResources/StandardMacros.DoOnce` false
    (:`Completed`
      (`GameplayStatics.PlaySoundAtLocation` "/Game/Audio/AudioClips/SFX/Chest_Open_Sound_Effect.Chest_Open_Sound_Effect" (`self.K2_GetActorLocation`) (struct) 1.0 1.0 0.0 null null null null))))

(fn `UserConstructionScript`
  (`KismetSystemLibrary.DrawDebugSphere` (`SceneComponent.K2_GetComponentLocation` (`self.Loot Spawn Point`)) 550.0 12 (struct :`R` 1.0 :`G` 1.0 :`B` 1.0 :`A` 1.0) 0.0 2.0))