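; BP_UnlockableWall is an interactable wall that opens when the player holds a key of the matching type.
; On Interact it loops through the player pawn's BP_InventoryComponent key list, comparing each key's enum to the wall's KeyType.
; A match disables the Glass collision and switches the front and back hieroglyph meshes to an emissive green material, while mismatches only reach a silent placeholder print.
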(event `/Game/Player/Interaction/BPI_Interactable.Interact`
  (`self.Compare Key Values`))

(fn `Compare Key Values`
  (for _array_element (`/Game/Components/BP_InventoryComponent.List of Keys` (`self.GetComponentByClass` (`GameplayStatics.GetPlayerPawn` 0) "/Game/Components/BP_InventoryComponent.BP_InventoryComponent_C"))
    (if (`|EnumEquality` (`/Game/Player/Inventory/Keys/PDA_Keys.Key Enum` _array_element) (`self.Key Type`))
      (`self.Unlock Wall`)
      (else
        (`KismetSystemLibrary.PrintString` "" false false) ; Handle incorrect key type here
      ))))

(fn `Unlock Wall`
  (`PrimitiveComponent.SetCollisionEnabled` (`self.Glass`) "NoCollision")
  (`PrimitiveComponent.SetMaterial` (`self.Hieroglyph Mesh Front`) 0 "/Game/Art/Materials/M_EmissiveGreen_Inst.M_EmissiveGreen_Inst")
  (`PrimitiveComponent.SetMaterial` (`self.Hieroglyph Mesh Back`) 0 "/Game/Art/Materials/M_EmissiveGreen_Inst.M_EmissiveGreen_Inst"))

(fn `UserConstructionScript`)