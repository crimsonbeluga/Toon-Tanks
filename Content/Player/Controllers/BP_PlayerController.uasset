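; Player controller that routes Enhanced Input to the possessed BP_PlayerPawn and owns the player's HUD and inventory widgets.
; On possession it caches the pawn, adds the input mapping, moves the audio listener to the pawn's SoundListener and rebuilds the HUD.
; Fire, move, look and interact forward to pawn handlers, while holding the inventory input shows the inventory.
; HUD rebuilds create a new inventory widget without removing the old one.
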(event `self.ReceiveBeginPlay`
  (`self.SetupDefaultInputMapping`)
  (`self.Initialize Player Hud`))

(event `self.ReceivePossess`
  (params (PossessedPawn :type "Pawn Object Reference"))
  (bind _asbp_player_pawn (cast `/Game/Player/Pawns/BP_PlayerPawn` PossessedPawn))
  (set `self.BP_Player Pawn Reference` _asbp_player_pawn)
  (`self.SetupDefaultInputMapping`)
  (`self.SetAudioListenerOverride` (`/Game/Player/Pawns/BP_PlayerPawn.Sound Listener` (`self.BP_Player Pawn Reference`)))
  (`self.Remove Player Hud`)
  (`self.Initialize Player Hud`))

(event `self.ReceiveUnPossess`
  (params (UnpossessedPawn :type "Pawn Object Reference"))
  (set `self.BP_Player Pawn Reference` null))

(event `EnhancedInput|/Game/Player/Input/Inputs/IA_Fire`
  (params (ActionValue :type Boolean) (ElapsedSeconds :type "Float (double-precision)") (TriggeredSeconds :type "Float (double-precision)") (InputAction :type "InputAction Object Reference" :default "/Game/Player/Input/Inputs/IA_Fire.IA_Fire"))
  (:`Started`
    (`/Game/Player/Pawns/BP_PlayerPawn.Handle Fire Pressed` (`self.BP_Player Pawn Reference`)))
  (:`Canceled`
    (`/Game/Player/Pawns/BP_PlayerPawn.Handle Fire Released` (`self.BP_Player Pawn Reference`) :!label _label))
  (:`Completed`
    (goto _label)))

(event `EnhancedInput|/Game/Player/Input/Inputs/IA_Move`
  (params (ActionValue :type "Vector2D Structure") (ElapsedSeconds :type "Float (double-precision)") (TriggeredSeconds :type "Float (double-precision)") (InputAction :type "InputAction Object Reference" :default "/Game/Player/Input/Inputs/IA_Move.IA_Move"))
  (:`Triggered`
    (`/Game/Player/Pawns/BP_PlayerPawn.Handle Move` (`self.BP_Player Pawn Reference`) ActionValue)))

(event `EnhancedInput|/Game/Player/Input/Inputs/IA_Look`
  (params (ActionValue :type "Vector2D Structure") (ElapsedSeconds :type "Float (double-precision)") (TriggeredSeconds :type "Float (double-precision)") (InputAction :type "InputAction Object Reference" :default "/Game/Player/Input/Inputs/IA_Look.IA_Look"))
  (:`Triggered`
    (`/Game/Player/Pawns/BP_PlayerPawn.Handle Look` (`self.BP_Player Pawn Reference`) 0.0)))

(event `EnhancedInput|/Game/Player/Input/Inputs/IA_Interact`
  (params (ActionValue :type Boolean) (ElapsedSeconds :type "Float (double-precision)") (TriggeredSeconds :type "Float (double-precision)") (InputAction :type "InputAction Object Reference" :default "/Game/Player/Input/Inputs/IA_Interact.IA_Interact"))
  (:`Started`
    (`/Game/Player/Pawns/BP_PlayerPawn.Handle Interaction` (`self.BP_Player Pawn Reference`))))

(event `EnhancedInput|/Game/Player/Input/Inputs/IA_Inventory`
  (params (ActionValue :type Boolean) (ElapsedSeconds :type "Float (double-precision)") (TriggeredSeconds :type "Float (double-precision)") (InputAction :type "InputAction Object Reference" :default "/Game/Player/Input/Inputs/IA_Inventory.IA_Inventory"))
  (:`Started`
    (`self.Show Inventory Widget`))
  (:`Completed`
    (`self.Hide Inventory Widget`)))

(event `Initialize Player Hud`
  (bind _returnvalue (`|CreateWidget` "/Game/UI/WBP_HUD.WBP_HUD_C"))
  (bind _output_get (set `self.HUD Widget` _returnvalue))
  (`UserWidget.AddToViewport` _output_get 0)
  (`self.Create Invetory Widget`))

(event `Remove Player Hud`
  (`Widget.RemoveFromParent` (`self.HUD Widget`)))

(event `Create Invetory Widget`
  (bind _returnvalue (`|CreateWidget` "/Game/UI/WBP_Inventory.WBP_Inventory_C"))
  (bind _output_get (set `self.Inventory Widget` _returnvalue))
  (`UserWidget.AddToViewport` _output_get 0)
  (`Widget.SetVisibility` (`self.Inventory Widget`) "Hidden"))

(event `Show Inventory Widget`
  (`Widget.SetVisibility` (`self.Inventory Widget`) "Visible"))

(event `Hide Inventory Widget`
  (`Widget.SetVisibility` (`self.Inventory Widget`) "Hidden"))

(fn `Remove Input Mapping`
  (`EnhancedInputSubsystemInterface.RemoveMappingContext` (subsystem `EnhancedInputLocalPlayerSubsystem`) (`self.IMC_Player`) (struct)))

(fn `SetupDefaultInputMapping`
  (`EnhancedInputSubsystemInterface.AddMappingContext` (subsystem `EnhancedInputLocalPlayerSubsystem`) (`self.IMC_Player`) 0 (struct)))

(fn `UserConstructionScript`)