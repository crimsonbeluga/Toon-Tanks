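; Player pawn with a cursor-aimed turret, weapon firing and proximity interaction.
; Move and fire handlers apply control-yaw-relative movement and forward triggers to BPWeaponComponent, whose equip event sets camera arm length.
; Tick eases turret yaw toward the cursor hit point and draws the interaction radius as a debug sphere.
; Radius overlaps track BPI_Interactable actors and toggle pickup prompts; interaction messages every tracked actor.
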(event `self.ReceiveTick`
  (params (DeltaSeconds :type "Float (single-precision)"))
  (bind _interactable_radius (`self.Interactable Radius`))
  (`self.Handle Look` DeltaSeconds)
  (`KismetSystemLibrary.DrawDebugSphere` (`SceneComponent.K2_GetComponentLocation` _interactable_radius) (`SphereComponent.SphereRadius` _interactable_radius) 12 (struct :`G` 1.0 :`B` 0.229393 :`A` 1.0) 0.1 1.0))

(event `self.Interactable Radius.OnComponentBeginOverlap`
  (params (OverlappedComponent :type "PrimitiveComponent Object Reference") (OtherActor :type "Actor Object Reference") (OtherComp :type "PrimitiveComponent Object Reference") (OtherBodyIndex :type Integer) (bFromSweep :type Boolean) (SweepResult :type "HitResult Structure (by ref)"))
  (`self.Handle Adding Interactable Actors` OverlappedComponent OtherActor OtherComp))

(event `self.Interactable Radius.OnComponentEndOverlap`
  (params (OverlappedComponent :type "PrimitiveComponent Object Reference") (OtherActor :type "Actor Object Reference") (OtherComp :type "PrimitiveComponent Object Reference") (OtherBodyIndex :type Integer))
  (`self.Handle Removing Interactable Actors` OverlappedComponent OtherActor OtherComp))

(event `self.ReceiveBeginPlay`
  (add `/Game/Components/BP_WeaponComponent.Equip Weapon` (`self.BP_WeaponComponent`) (delegate `Change Camera Positioning Based on Weapon`)))

(event `Change Camera Positioning Based on Weapon`
  (set `SpringArmComponent.TargetArmLength` (`/Game/Weapons/WeaponData/DA_WeaponDefintion.Camera Offset` (`/Game/Components/BP_WeaponComponent.Current Weapon Data` (`self.BP_WeaponComponent`))) (`self.SpringArm`)))

(fn `Handle Adding Interactable Actors`
  (params (`Input Overlapped Component` :type "PrimitiveComponent Object Reference") (`Input Other Actor` :type "Actor Object Reference") (`Input Other Component` :type "PrimitiveComponent Object Reference"))
  (locals (`Overlapped Component` :type "PrimitiveComponent Object Reference") (`Other Actor` :type "Actor Object Reference") (`Other Component` :type "PrimitiveComponent Object Reference"))
  (set `local.Overlapped Component` `Input Overlapped Component`)
  (set `local.Other Actor` `Input Other Actor`)
  (set `local.Other Component` `Input Other Component`)
  (if (== (`local.Overlapped Component`) (`self.Interactable Radius`))
    (if (`KismetSystemLibrary.DoesImplementInterface` (`local.Other Actor`) "/Game/Core/Interfaces/BPI_Interactable.BPI_Interactable_C")
      (`KismetArrayLibrary.Array_Add` (`self.Interactable Actors`) (`local.Other Actor`))
      (bind _asbp_interactable_pickup_base (cast `/Game/Environment/Interactabke/BP_InteractablePickupBase` (`local.Other Actor`)))
      (`/Game/Environment/Interactabke/BP_InteractablePickupBase.Show Interact UI` _asbp_interactable_pickup_base))))

(fn `Handle Fire Pressed`
  (`/Game/Components/BP_WeaponComponent.On Fire Pressed ` (`self.BP_WeaponComponent`)))

(fn `Handle Fire Released`
  (`/Game/Components/BP_WeaponComponent.On Fire Released` (`self.BP_WeaponComponent`)))

(fn `Handle Interaction`
  (for _array_element (`self.Interactable Actors`)
    (`/Engine/EditorBlueprintResources/StandardMacros.IsValid` _array_element
      (:`Is Valid`
        (message `/Game/Core/Interfaces/BPI_Interactable.Interact` _array_element self)
        (bind _asbp_interactable_pickup_base (cast `/Game/Environment/Interactabke/BP_InteractablePickupBase` _array_element))
        (`/Game/Environment/Interactabke/BP_InteractablePickupBase.Hide Interact UI` _asbp_interactable_pickup_base)
        (set `/Game/Environment/Interactabke/BP_InteractablePickupBase.bCanShowUI` false _asbp_interactable_pickup_base)))))

(fn `Handle Look`
  (params (`Delta Time` :type "Float (double-precision)"))
  (locals (`Current Mouse Location` :type "Vector Structure" :default (0.0 0.0 0.0)) (`Look At Rotation` :type "Rotator Structure") (`Local Delta Time` :type "Float (double-precision)"))
  (bind (_returnvalue_roll _returnvalue_pitch _returnvalue_yaw) (`KismetMathLibrary.BreakRotator` (`KismetMathLibrary.FindLookAtRotation` (`SceneComponent.K2_GetComponentLocation` (`self.Muzzle`)) (`local.Current Mouse Location`))))
  (set `local.Local Delta Time` `Delta Time`)
  (set `local.Current Mouse Location` (`.ImpactPoint` (`GameplayStatics.BreakHitResult` (`PlayerController.GetHitResultUnderCursorByChannel` (`GameplayStatics.GetPlayerController` 0) "TraceTypeQuery1" true))))
  (set `local.Look At Rotation` (`KismetMathLibrary.MakeRotator` 0.0 0.0 _returnvalue_yaw))
  (`SceneComponent.K2_SetWorldRotation` (`self.Turret`) (`KismetMathLibrary.RInterpTo` (`SceneComponent.K2_GetComponentRotation` (`self.Turret`)) (`local.Look At Rotation`) (`local.Local Delta Time`) (`self.TurretRotationSpeed`)) false false))

(fn `Handle Move`
  (params (`Movement Input vector` :type "Vector2D Structure"))
  (locals (`Movement Input Vector X` :type "Float (double-precision)" :default 0.0) (`Movement Inpute Vector Y` :type "Float (double-precision)" :default 0.0) (`Current Player Rotation` :type "Rotator Structure"))
  (bind (_returnvalue_roll _returnvalue_pitch _returnvalue_yaw) (`KismetMathLibrary.BreakRotator` (`Controller.GetControlRotation` (`GameplayStatics.GetPlayerController` 0))))
  (set `local.Movement Input Vector X` `Movement Input vector_X`)
  (set `local.Movement Inpute Vector Y` `Movement Input vector_Y`)
  (bind _output_get (set `local.Current Player Rotation` (`KismetMathLibrary.MakeRotator` 0.0 0.0 _returnvalue_yaw)))
  (`self.AddMovementInput` (`KismetMathLibrary.GetForwardVector` _output_get) (`local.Movement Input Vector X`))
  (`self.AddMovementInput` (`KismetMathLibrary.GetRightVector` _output_get) (`local.Movement Inpute Vector Y`)))

(fn `Handle Removing Interactable Actors`
  (params (`Input Overlapped Component` :type "PrimitiveComponent Object Reference") (`Input Other Actor` :type "Actor Object Reference") (`Input Other Component` :type "PrimitiveComponent Object Reference"))
  (locals (`Array Index` :type Integer) (`Array Element` :type "Actor Object Reference") (`Overlapped Component` :type "PrimitiveComponent Object Reference") (`Other Component` :type "PrimitiveComponent Object Reference") (`Other Actor` :type "Actor Object Reference"))
  (set `local.Overlapped Component` `Input Overlapped Component`)
  (set `local.Other Actor` `Input Other Actor`)
  (set `local.Other Component` `Input Other Component`)
  (if (`PrimitiveComponent.IsOverlappingActor` (`self.Interactable Radius`) (`local.Other Actor`))
    _
    (elif (== (`local.Overlapped Component`) (`self.Interactable Radius`))
      (for (_array_element _array_index) (`self.Interactable Actors`)
        (set `local.Array Element` _array_element)
        (set `local.Array Index` _array_index)
        (if (== (`local.Other Actor`) (`local.Array Element`))
          (set `local.Array Element` null)
          (`KismetArrayLibrary.Array_Remove` (`self.Interactable Actors`))
          (bind _asbp_interactable_pickup_base (cast `/Game/Environment/Interactabke/BP_InteractablePickupBase` (`local.Other Actor`)))
          (`/Game/Environment/Interactabke/BP_InteractablePickupBase.Hide Interact UI` _asbp_interactable_pickup_base))))))

(fn `UserConstructionScript`)