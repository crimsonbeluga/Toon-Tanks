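; BP_BaseProjectile is a base weapon projectile that damages what it overlaps through that actor's health component.
; On BeginPlay its collision box ignores the instigator and owner when moving.
; On overlap it skips the owner, looks up BP_HealthComponent on the other actor and applies Damage if found.
; It destroys itself after any non-owner overlap, with or without a health component, and prints debug messages.
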(event `self.ReceiveBeginPlay`
  (`PrimitiveComponent.IgnoreActorWhenMoving` (`self.Collision Box`) (`self.GetInstigator`) true)
  (`PrimitiveComponent.IgnoreActorWhenMoving` (`self.Collision Box`) (`self.GetOwner`) true))

(event `self.Collision Box.OnComponentBeginOverlap`
  (params (OverlappedComponent :type "PrimitiveComponent Object Reference") (OtherActor :type "Actor Object Reference") (OtherComp :type "PrimitiveComponent Object Reference") (OtherBodyIndex :type Integer) (bFromSweep :type Boolean) (SweepResult :type "HitResult Structure (by ref)"))
  (if (== OtherActor (`self.GetOwner`))
    (`KismetSystemLibrary.PrintString` "BP_BaseProjectle - On COmponent Begin Overlap: We hit Are selves" false false)
    (else
      (bind _output_get (set `self.Other Actor` OtherActor))
      (bind _output_get_2 (set `self.BP_Health Component Reference` (`self.GetComponentByClass` _output_get "/Game/Components/BP_HealthComponent.BP_HealthComponent_C")))
      (if (`KismetSystemLibrary.IsValid` _output_get_2)
        (`/Game/Components/BP_HealthComponent.ApplyDamage` (`self.BP_Health Component Reference`) (`self.Damage`))
        (`self.K2_DestroyActor`)
        (`KismetSystemLibrary.PrintString` "We have made it all the way through ")
        (else
          (`KismetSystemLibrary.PrintString` "BP_Projectile  - On Component Begin Overlap: the health component reference is not valid or null So we are destroying the Actor")
          (`self.K2_DestroyActor`))))))

(fn `UserConstructionScript`)